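; OrbActor2 is a collectible orb that MyCharacter picks up on overlap.
; Overlap increments the character's OrbsCollected, sets ShowOrbCollectedTint for a short Delay, then clears it and destroys the orb.
; Nothing disables overlap during that delay, so re-entering can count the orb again.
; A Timeline meant to yaw the Sphere is never started, so the orb does not spin through this graph.
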(event `self.ReceiveActorBeginOverlap`
  (params (OtherActor :type "Actor Object Reference"))
  (bind _asmy_character (cast `/Game/MyContent/MyCharacter` OtherActor))
  (set `/Game/MyContent/MyCharacter.OrbsCollected` (+ (`/Game/MyContent/MyCharacter.OrbsCollected` _asmy_character) 1) _asmy_character)
  (set `/Game/MyContent/MyCharacter.ShowOrbCollectedTint` true _asmy_character)
  (`KismetSystemLibrary.Delay` 0.3)
  (set `/Game/MyContent/MyCharacter.ShowOrbCollectedTint` false _asmy_character)
  (`self.K2_DestroyActor`))

(fn `UserConstructionScript`)