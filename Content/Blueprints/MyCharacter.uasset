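; MyCharacter is the player character Blueprint, handling health, a timed Clear Vision power, and the HUD, pause, game-over and win screens.
; BeginPlay creates the widgets, and the game-over and win events swap in their menu, switch to UI-only input and pause.
; Damage passes through a DoOnce that resets after a delayed tint flag, while depleted health calls the win event.
; Clear Vision temporarily overrides camera post-processing, then restores it.
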(event `self.ReceiveBeginPlay`
  ;[1 1 1] Create HUD and Menu widgets
  (bind _returnvalue (`|CreateWidget` "/Game/Blueprints/MyHUD.MyHUD_C"))
  (bind _output_get (set `self.MyHUD` _returnvalue))
  (`UserWidget.AddToViewport` _output_get 0)
  (bind _returnvalue_2 (`|CreateWidget` "/Game/Blueprints/PauseMenu.PauseMenu_C"))
  (set `self.PauseMenu` _returnvalue_2)
  (bind _returnvalue_3 (`|CreateWidget` "/Game/Blueprints/GameOverMenu.GameOverMenu_C"))
  (set `self.GameOverMenu` _returnvalue_3)
  (bind _returnvalue_4 (`|CreateWidget` "/Game/Blueprints/WinScreenMenu.WinScreenMenu_C"))
  (set `self.WinScreenMenu` _returnvalue_4))

(event `EventGameOver`
  (bind _returnvalue (`GameplayStatics.GetPlayerController` 0))
  (bind _gameovermenu (`self.GameOverMenu`))
  ;[1 1 1] Game Over
  (`WidgetLayoutLibrary.RemoveAllWidgets`)
  (`UserWidget.AddToViewport` _gameovermenu 0)
  (`WidgetBlueprintLibrary.SetInputMode_UIOnlyEx` _returnvalue _gameovermenu)
  (set `PlayerController.bShowMouseCursor` true _returnvalue)
  (`GameplayStatics.SetGamePaused` true))

(event `ActivatePower`
  (params (PowerName :type String))
  (`KismetSystemLibrary.PrintString` "Activating Clear Vision")
  (set `self.HasClearVisionPower` true)
  (bind _output_get (set `self.InitialPostProcessSettings` (`CameraComponent.PostProcessSettings` (`self.Camera`))))
  (set `CameraComponent.PostProcessSettings` (make `PostProcessSettings` :`AutoExposureMaxBrightness` 0.04) (`self.Camera`))
  (`KismetSystemLibrary.Delay` 5.0)
  (set `self.HasClearVisionPower` false)
  (set `CameraComponent.PostProcessSettings` _output_get (`self.Camera`)))

(event `EventWinGame`
  (bind _returnvalue (`GameplayStatics.GetPlayerController` 0))
  (bind _winscreenmenu (`self.WinScreenMenu`))
  ;[1 1 1] Win Game
  (`WidgetLayoutLibrary.RemoveAllWidgets`)
  (`UserWidget.AddToViewport` _winscreenmenu 0)
  (`WidgetBlueprintLibrary.SetInputMode_UIOnlyEx` _returnvalue _winscreenmenu)
  (set `PlayerController.bShowMouseCursor` true _returnvalue)
  (`GameplayStatics.SetGamePaused` true))

(event `self.ReceiveAnyDamage`
  (params (Damage :type "Float (single-precision)") (DamageType :type "DamageType Object Reference") (InstigatedBy :type "Controller Object Reference") (DamageCauser :type "Actor Object Reference"))
  ;[1 1 1] Deducts Health
  (`/Engine/EditorBlueprintResources/StandardMacros.DoOnce` false :!label _label
    (:`Completed`
      (bind _output_get (set `self.Health` (- (`self.Health`) Damage)))
      (if (<= _output_get 0.001)
        (`self.EventWinGame`)
        (else
          (set `self.ShowDamageTint` true)
          (`KismetSystemLibrary.Delay` 0.3)
          (set `self.ShowDamageTint` false)
          (`KismetSystemLibrary.Delay` 0.2)
          (goto _label :!via `Reset`))))))

(fn `UserConstructionScript`)